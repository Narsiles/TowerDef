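; BP_Boat is an enemy boat that travels along a spline and can be destroyed by towers for gold and score.
; Its Type selects mesh, health and score value, and a world-facing life bar widget turns toward the player camera each tick.
; A Timeline drives position and rotation along the spline, with play rate set from player score so higher scores give faster boats.
; On lethal damage, it clears the tower's boat reference, rewards the player and destroys itself.
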(event `SetTimeSec`
  ;[0.2097 1 0] Set un nouveau temps en seconde celon le score actuelle in game
  (`TimelineComponent.SetPlayRate` (`self.Timeline`) (/ 1.0 (`KismetMathLibrary.MapRangeClamped` (`/Game/Blueprint/BP_Player.Score` (`self.As BP Player`)) 0.0 1000.0 30.0 5.0))))

(event `self.ReceiveBeginPlay`
  (bind _splinetofollow (`self.SplineToFollow`))
  ;[1 0.3556 0.2155] Initialisation Boat/Widget/FollowSpline
  (`self.InitBoat`)
  (bind _asbp_player (cast `/Game/Blueprint/BP_Player` (`GameplayStatics.GetPlayerPawn` 0)))
  (set `self.As BP Player` _asbp_player)
  (bind _aswg_life_bar (cast `/Game/UI/WG_LifeBar` (`WidgetComponent.GetWidget` (`self.Widget`))))
  (set `/Game/UI/WG_LifeBar.Boat` self _aswg_life_bar)
  (`self.SetTimeSec`)
  (bind (_direction _newtrack_0) (`Timeline|Timeline`)
    (:`Update`
      (bind _returnvalue (`KismetMathLibrary.Lerp` 0.0 (`SplineComponent.GetSplineLength` _splinetofollow) (- 1.0 _newtrack_0)))
      (bind (_returnvalue_roll _returnvalue_pitch _returnvalue_yaw) (`KismetMathLibrary.BreakRotator` (`SplineComponent.GetRotationAtDistanceAlongSpline` _splinetofollow _returnvalue "Local")))
      (`self.K2_SetActorTransform` self (`KismetMathLibrary.MakeTransform` (`SplineComponent.GetLocationAtDistanceAlongSpline` _splinetofollow _returnvalue "World") (`KismetMathLibrary.MakeRotator` _returnvalue_roll _returnvalue_pitch (+ _returnvalue_yaw 90.0))) false false))))

(event `self.ReceiveAnyDamage`
  (params (Damage :type "Float (single-precision)") (DamageType :type "DamageType Object Reference") (InstigatedBy :type "Controller Object Reference") (DamageCauser :type "Actor Object Reference"))
  (bind _as_bp_player (`self.As BP Player`))
  ;[0.89 0.1682 1] Prise de dommage
  (bind _output_get (set `self.LifePoint` (- (`self.LifePoint`) Damage)))
  (if (<= _output_get 0.0)
    (bind _asbp_tower (cast `/Game/Blueprint/BP_Tower` DamageCauser))
    (set `/Game/Blueprint/BP_Tower.As BP Boat` null _asbp_tower)
    (set `/Game/Blueprint/BP_Player.Gold` (+ (`/Game/Blueprint/BP_Player.Gold` _as_bp_player) 5.0) _as_bp_player)
    (set `/Game/Blueprint/BP_Player.Score` (+ (`/Game/Blueprint/BP_Player.Score` _as_bp_player) (`self.ScoreB`)) _as_bp_player)
    (`self.SetTimeSec`)
    (`self.K2_DestroyActor`)))

(event `InitBoat`
  (bind _type (`self.Type`))
  (bind _returnvalue (select `int` _type :`0` 15.0 :`1` 20.0 :`2` 35.0))
  ;[0.2488 0.295 1] Selection de bateau aléatoire entre trois type
  (set `self.LifePointMax` _returnvalue)
  (set `self.LifePoint` _returnvalue)
  (set `self.ScoreB` (select `int` _type :`0` 1.0 :`1` 2.0 :`2` 3.0))
  (`StaticMeshComponent.SetStaticMesh` (`self.StaticMesh`) (select `int` _type :`0` "/Game/MeshAnto/MainMeshes/SM_Petit_Bateau.SM_Petit_Bateau" :`1` "/Game/MeshAnto/MainMeshes/SM_MoyenBateau.SM_MoyenBateau" :`2` "/Game/MeshAnto/MainMeshes/SM_GrosBateau.SM_GrosBateau" :!type "StaticMesh Object Reference")))

(event `self.ReceiveTick`
  (params (DeltaSeconds :type "Float (single-precision)"))
  ;[0.9985 1 0.3514] Barre de vie actualisation
  (`SceneComponent.K2_SetWorldRotation` (`self.Widget`) (`KismetMathLibrary.FindLookAtRotation` (`SceneComponent.K2_GetComponentLocation` (`self.Widget`)) (`SceneComponent.K2_GetComponentLocation` (`/Game/Blueprint/BP_Player.Camera` (`self.As BP Player`)))) false false))

(fn `UserConstructionScript`)