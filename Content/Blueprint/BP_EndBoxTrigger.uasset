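; BP_EndBoxTrigger is a box trigger that costs the player a life when something, labeled as a boat, reaches it.
; It caches the BP_Player pawn on BeginPlay.
; On overlap it subtracts one from that player's Life while above zero, then destroys the overlapping actor.
; The overlap branch is hardwired true, so any actor entering the box triggers both effects without a type check.
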(event `self.ReceiveBeginPlay`
  ;[1 1 1] Get player ref
  (bind _asbp_player (cast `/Game/Blueprint/BP_Player` (`GameplayStatics.GetPlayerPawn` 0)))
  (set `self.As BP Player` _asbp_player))

(event `Remove Life`
  (bind _as_bp_player (`self.As BP Player`))
  (bind _life (`/Game/Blueprint/BP_Player.Life` _as_bp_player))
  ;[1 1 1] Remove Life
  (if (> _life 0.0)
    (set `/Game/Blueprint/BP_Player.Life` (- _life 1.0) _as_bp_player)))

(event `self.Box.OnComponentBeginOverlap`
  (params (OverlappedComponent :type "PrimitiveComponent Object Reference") (OtherActor :type "Actor Object Reference") (OtherComp :type "PrimitiveComponent Object Reference") (OtherBodyIndex :type Integer) (bFromSweep :type Boolean) (SweepResult :type "HitResult Structure (by ref)"))
  ;[1 1 1] BoatOverlap
  (if true
    (`self.Remove Life`)
    (`self.K2_DestroyActor` OtherActor)))

(fn `UserConstructionScript`)