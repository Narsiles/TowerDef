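; BP_Player is the player pawn for a tower defense game, handling camera movement and gold-based turret placement.
; On possession it adds the IMC_Player Enhanced Input context, and IA_Move drives movement along fixed world axes.
; IA_ValidTower spawns the selected tower class at the cursor's Visibility hit when a separate blocking-channel trace misses and Gold exceeds its GlobalCost, then deducts that cost.
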(event `self.ReceivePossessed`
  (params (NewController :type "Controller Object Reference"))
  ;[1 0.3932 0.7422] Mapping
  (bind _asplayer_controller (cast `PlayerController` NewController))
  (bind _returnvalue (pcsubsystem `EnhancedInputLocalPlayerSubsystem` _asplayer_controller))
  (`/Engine/EditorBlueprintResources/StandardMacros.IsValid` _returnvalue
    (:`Is Valid`
      (`EnhancedInputSubsystemInterface.AddMappingContext` _returnvalue "/Game/Blueprint/Input/IMC_Player.IMC_Player" 0 (struct)))))

(event `EnhancedInput|/Game/Blueprint/Input/InputAction/IA_Move`
  (params (ActionValue :type "Vector2D Structure") (ElapsedSeconds :type "Float (double-precision)") (TriggeredSeconds :type "Float (double-precision)") (InputAction :type "InputAction Object Reference" :default "/Game/Blueprint/Input/InputAction/IA_Move.IA_Move"))
  ;[1 0.3082 0.01503] Movement Cam
  (:`Triggered`
    (`|ExecutionSequence`
      (:`then_0`
        (`self.AddMovementInput` (1.0 0.0 0.0) ActionValue_Y))
      (:`then_1`
        (`self.AddMovementInput` (0.0 -1.0 0.0) ActionValue_X)))))

(event `EnhancedInput|/Game/Blueprint/Input/InputAction/IA_ValidTower`
  (params (ActionValue :type Boolean) (ElapsedSeconds :type "Float (double-precision)") (TriggeredSeconds :type "Float (double-precision)") (InputAction :type "InputAction Object Reference" :default "/Game/Blueprint/Input/InputAction/IA_ValidTower.IA_ValidTower"))
  (bind _gold (`self.Gold`))
  (bind _value (`BlueprintMapLibrary.Map_Find` (`self.GlobalCost`) (`self.SelectedTower`)))
  ;[0.4214 0.775 1] Placer  une tourelle
  (:`Started`
    (if (`GameplayStatics.BreakHitResult` (`PlayerController.GetHitResultUnderCursorByChannel` (`GameplayStatics.GetPlayerController` 0) "TraceTypeQuery3" true))
      _
      (elif (> _gold _value)
        (`|SpawnActorFromClass` (select `/Game/Blueprint/TowerType` (`self.SelectedTower`) :`NewEnumerator0` "/Game/Blueprint/BP_TowerCac.BP_TowerCac_C" :`NewEnumerator1` "/Game/Blueprint/BP_TowerRange.BP_TowerRange_C" :`NewEnumerator2` "/Game/Blueprint/BP_TowerMid.BP_TowerMid_C" :!type "Actor Class Reference") (`KismetMathLibrary.MakeTransform` (`.Location` (`GameplayStatics.BreakHitResult` (`PlayerController.GetHitResultUnderCursorByChannel` (`GameplayStatics.GetPlayerController` 0) "TraceTypeQuery1" true)))) "Undefined" "OverrideRootScale" null null)
        (set `self.Gold` (- _gold _value))))))

(fn `UserConstructionScript`)