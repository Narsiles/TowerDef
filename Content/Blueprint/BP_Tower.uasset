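; BP_Tower is a defensive tower that automatically damages BP_Boat actors within its range sphere.
; Tick targets the first overlapping boat and, when enabled, smoothly yaws toward it.
; A looping timer set at BeginPlay damages that target or all overlapping boats, depending on AttackAll.
; The construction script sizes the range sphere and spacing box; Upgrade raises the Range and AttackSpeed variables at level 2 without refreshing the sphere or timer.
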(event `self.ReceiveBeginPlay`
  ;[1 1 1] Application des dommages
  (`KismetSystemLibrary.K2_SetTimerDelegate` (delegate `Attack`) (`self.AttackSpeed`) true))

(event `Attack`
  ;[1 1 1] Application des dommages
  (`/Engine/EditorBlueprintResources/StandardMacros.IsValid` (`self.As BP Boat`)
    (:`Is Valid`
      (if (`self.shouldAttack`)
        (if (`self.AttackAll`)
          (for _array_element (`self.Overlapping Actors`)
            (`GameplayStatics.ApplyDamage` _array_element (`self.Dammage`) null self))
          (else
            (`GameplayStatics.ApplyDamage` (`self.As BP Boat`) (`self.Dammage`) null self)))))))

(event `self.ReceiveTick`
  (params (DeltaSeconds :type "Float (single-precision)"))
  ;[1 1 1] Detection du premier bateau
  (bind _output_get (set `self.Overlapping Actors` (`PrimitiveComponent.GetOverlappingActors` (`self.RangeDetection`) "/Game/Blueprint/BP_Boat.BP_Boat_C")))
  (bind _asbp_boat (cast `/Game/Blueprint/BP_Boat` (`|GetArrayItem` _output_get)))
  (set `self.As BP Boat` _asbp_boat)
  (`self.FaceEnemy`))

(event `FaceEnemy`
  (bind (_returnvalue_roll _returnvalue_pitch _returnvalue_yaw) (`KismetMathLibrary.BreakRotator` (`KismetMathLibrary.RInterpTo` (`self.K2_GetActorRotation`) (`KismetMathLibrary.FindLookAtRotation` (`self.K2_GetActorLocation`) (`self.K2_GetActorLocation` (`self.As BP Boat`))) (`GameplayStatics.GetWorldDeltaSeconds`) 10.0)))
  ;[1 1 1] FaceEnemy
  (if (`self.shouldRotate`) :!label _label
    (`self.As BP Boat`
      (:`then`
        (`self.K2_SetActorRotation` (`KismetMathLibrary.MakeRotator` 0.0 0.0 _returnvalue_yaw)))
      (:`else`))))

(event `self.Sphere.OnComponentBeginOverlap`
  (params (OverlappedComponent :type "PrimitiveComponent Object Reference") (OtherActor :type "Actor Object Reference") (OtherComp :type "PrimitiveComponent Object Reference") (OtherBodyIndex :type Integer) (bFromSweep :type Boolean) (SweepResult :type "HitResult Structure (by ref)"))
  ;[1 1 1] FaceEnemy
  (goto _label))

(event `Upgrade`
  ;[1 1 1] Upgrade
  (if (== (`self.TowerLevel`) 2.0)
    (set `self.Range` (+ (`self.Range`) 1000.0))
    (set `self.AttackSpeed` (+ (`self.AttackSpeed`) 0.4))))

(fn `UserConstructionScript`
  (`SphereComponent.SetSphereRadius` (`self.RangeDetection`) (`self.Range`) true)
  (`BoxComponent.SetBoxExtent` (`self.SpaceInBetweenBox`) (`KismetMathLibrary.Conv_DoubleToVector` (`self.BetweenSpace`)) true))